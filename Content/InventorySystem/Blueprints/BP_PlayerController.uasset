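; BP_PlayerController is the player controller that turns input axes into movement and camera look for BP_PlayerCharacter.
; On possess it casts the pawn and caches it as CharacterReference, which every input handler validates before use.
; Forward and right movement follow the control rotation's yaw only and are blocked while IsMovementLocked is set.
; Turn and look-up input feed controller yaw and pitch and ignore that lock.
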(event EventBeginPlay)

(event EventTick
  (params (DeltaSeconds :type Float%20%28single-precision%29)))

(event EventPossess
  (params (PossessedPawn :type Pawn%20Object%20Reference))
  ;[1 1 1] Possess
  (bind _asbp_player_character (Utilities|Casting|CastToBP_PlayerCharacter PossessedPawn))
  (Variables|Default|SetCharacterReference _asbp_player_character))

(event Input|AxisEvents|InputAxisMoveForward
  (params (AxisValue :type Float%20%28single-precision%29))
  (bind _characterreference (Variables|Default|GetCharacterReference))
  ;[1 1 1] InputMove
  (if (not (Variables|Default|GetIsMovementLocked))
    (Utilities|IsValid _characterreference
      (:Is%20Valid
        (Pawn|Input|AddMovementInput _characterreference (Math|Vector|GetForwardVector (Math|Rotator|MakeRotator 0.0 0.0 (.Yaw (Math|Rotator|BreakRotator (Pawn|GetControlRotation :!class /Script/Engine.Controller))))) AxisValue false)))))

(event Input|AxisEvents|InputAxisMoveRight
  (params (AxisValue :type Float%20%28single-precision%29))
  (bind _characterreference (Variables|Default|GetCharacterReference))
  ;[1 1 1] InputMove
  (if (not (Variables|Default|GetIsMovementLocked))
    (Utilities|IsValid _characterreference
      (:Is%20Valid
        (Pawn|Input|AddMovementInput _characterreference (Math|Vector|GetRightVector (Math|Rotator|MakeRotator 0.0 0.0 (.Yaw (Math|Rotator|BreakRotator (Pawn|GetControlRotation :!class /Script/Engine.Controller))))) AxisValue false)))))

(event Input|AxisEvents|InputAxisTurn
  (params (AxisValue :type Float%20%28single-precision%29))
  (bind _characterreference (Variables|Default|GetCharacterReference))
  ;[1 1 1] Input Turn
  (Utilities|IsValid _characterreference
    (:Is%20Valid
      (Pawn|Input|AddControllerYawInput _characterreference AxisValue))))

(event Input|AxisEvents|InputAxisLookUp
  (params (AxisValue :type Float%20%28single-precision%29))
  (bind _characterreference (Variables|Default|GetCharacterReference))
  ;[1 1 1] Input Turn
  (Utilities|IsValid _characterreference
    (:Is%20Valid
      (Pawn|Input|AddControllerPitchInput _characterreference AxisValue))))

(fn ConstructionScript)