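; BP_Useable is a usable world actor in the inventory system that provides default responses for focus and use, apparently as a base to override.
; Focus functions toggle custom depth rendering on its StaticMesh to drive an outline highlight.
; It reports itself as usable with empty action and key text, while OnActorUsed takes a Controller and returns false without doing anything.
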(event EventBeginPlay)

(event Collision|EventActorBeginOverlap
  (params (OtherActor :type Actor%20Object%20Reference)))

(event EventTick
  (params (DeltaSeconds :type Float%20%28single-precision%29)))

(fn ConstructionScript)

(fn BeginOutlineFocus
  (Rendering|SetRenderCustomDepth (Variables|Default|GetStaticMesh) true)
  (return true))

(fn EndOutlineFocus
  (Rendering|SetRenderCustomDepth (Variables|Default|GetStaticMesh) false)
  (return true))

(fn GetIsActorUsable
  (return true))

(fn GetUseActionText
  (return ""))

(fn GetUseKeyText
  (return ""))

(fn OnActorUsed
  (params (Controller :type BP%20Player%20Controller%20Object%20Reference))
  (return false))